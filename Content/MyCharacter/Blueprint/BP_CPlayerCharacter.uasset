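; Player character Blueprint with weapon switching, three-hit combo attacks, sliding and vaulting.
; Fists or greatsword select the combo montages, and switching updates the attached mesh and UI text.
; Sliding shrinks the capsule, uses timed traces to align to slopes and stop at walls or ledges, and crouches under ceilings.
; Vaulting traces obstacle length and landing, feeds Motion Warping targets, and plays a random montage chosen by distance while in Flying mode.
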(event `self.ReceiveBeginPlay`)

(event `EnhancedInput|/Game/MyCharacter/Blueprint/Input/InputAction/IA_MoveAction`
  (params (ActionValue :type "Vector2D Structure") (ElapsedSeconds :type "Float (double-precision)") (TriggeredSeconds :type "Float (double-precision)") (InputAction :type "InputAction Object Reference" :default "/Game/MyCharacter/Blueprint/Input/InputAction/IA_MoveAction.IA_MoveAction"))
  (bind (_x _y) (`KismetMathLibrary.BreakVector2D` ActionValue))
  (:`Triggered`
    (`self.MoveActionFunc` (make `InputActionValue` _x _y 0.0 "Axis2D"))
    ;[1 1 1] If crouched after sliding under an object, then the trace will run everytime the player moves so that it will dtetect when they exit the object and can stand up again.
    (if (`self.Is Detect Ceiling`)
      (`self.Trace For Ceiling`))))

(event `self.ReceiveTick`
  (params (DeltaSeconds :type "Float (single-precision)")))

(event `Trace For Ceiling`
  (bind _returnvalue (`NavMovementComponent.IsCrouching` (`self.CharacterMovement`)))
  (bind _returnvalue_2 (+ (`self.K2_GetActorLocation`) (0.0 0.0 60.0)))
  (bind (_outhit _returnvalue_3) (`KismetSystemLibrary.CapsuleTraceSingle` _returnvalue_2 _returnvalue_2 34.0 88.0 "TraceTypeQuery1" false (`|MakeArray` null :!type "Actor Object Reference") "ForOneFrame"))
  (if _returnvalue_3
    (if (not _returnvalue)
      (`self.Crouch`)
      (`AnimInstance.Montage_Stop` (`SkeletalMeshComponent.GetAnimInstance` (`self.Mesh`)) 0.2 null)
      (set `self.Is Detect Ceiling` true))
    (elif _returnvalue
      (`self.UnCrouch`)
      (set `self.Is Detect Ceiling` false))))

(event `Reset XY Rotation`
  (bind (_returnvalue_roll _returnvalue_pitch _returnvalue_yaw) (`KismetMathLibrary.BreakRotator` (`self.K2_GetActorRotation`)))
  (bind _charactermovement (`self.CharacterMovement`))
  (set `self.Default Yaw Rotation` (`KismetMathLibrary.MakeRotator` 0.0 0.0 _returnvalue_yaw))
  (bind (_direction _value) (`Timeline|Reset Slide Rotation` :!via `PlayFromStart`)
    (:`Update`
      (`self.K2_SetActorRotation` (`KismetMathLibrary.RLerp` (`self.K2_GetActorRotation`) (`self.Default Yaw Rotation`) _value)))
    (:`Finished`
      (set `CharacterMovementComponent.MaxWalkSpeed` 500.0 _charactermovement)
      (set `CharacterMovementComponent.MaxAcceleration` 1500.0 _charactermovement))))

(event `Continue Sliding`
  (bind _angle (`self.FindCurrentFloorAngleAndDirection`))
  (bind (_returnvalue_roll _returnvalue_pitch _returnvalue_yaw) (`KismetMathLibrary.BreakRotator` (`self.K2_GetActorRotation`)))
  (bind _charactermovement (`self.CharacterMovement`))
  (bind _output_get (set `self.Current Angle` _angle))
  (if (< (`KismetMathLibrary.FInterpTo` _output_get _angle (`GameplayStatics.GetWorldDeltaSeconds`) 0.4) 3.0)
    (if (< (`KismetMathLibrary.VSize` (`MovementComponent.Velocity` (`self.CharacterMovement`))) (`self.Speed To Stop Sliding`))
      (`KismetSystemLibrary.K2_ClearAndInvalidateTimerHandle` (`self.Continue Sliding Handle`) :!label _label)
      (`self.Play GetUp Animation`))
    (else
      (`|ExecutionSequence`
        (:`then_0`
          (`self.AddMovementInput` (`KismetMathLibrary.GetForwardVector` (`KismetMathLibrary.MakeRotator` 0.0 0.0 _returnvalue_yaw)))
          (set `CharacterMovementComponent.MaxWalkSpeed` 1500.0 _charactermovement) ; What ther maximum speed reachable\nshould be when sliding at the fastest
          (set `CharacterMovementComponent.MaxAcceleration` 500.0 _charactermovement) ; Decides how fast or slow the change \nin speed is while sliding (how gradual it is)
        )
        (:`then_1`
          (`self.Check Hit Surface` 0.0
            (:`true`
              (goto _label))))))))

(event `Play GetUp Animation`
  (bind _slide_trace_handle (`self.Slide Trace Handle`))
  (`AnimInstance.Montage_Play` (`SkeletalMeshComponent.GetAnimInstance` (`self.Mesh`)) "/Game/MyCharacter/Animation/Montage/Sliding/AM_SlidingEnd.AM_SlidingEnd" 1.0 "MontageLength" 0.0 true :!label _label_2)
  (`KismetSystemLibrary.RetriggerableDelay` 0.02)
  (`|ExecutionSequence`
    (:`then_0`
      (if (`KismetSystemLibrary.K2_IsValidTimerHandle` _slide_trace_handle)
        (`KismetSystemLibrary.K2_ClearAndInvalidateTimerHandle` _slide_trace_handle)))
    (:`then_1`
      (`self.Revert Capsule`))
    (:`then_2`
      (`self.Reset XY Rotation`))))

(event `Check Should Continue Sliding`
  (if (`self.IsSliding`)
    (if (`.Is Slope Up` (`self.FindCurrentFloorAngleAndDirection`))
      (set `MovementComponent.Velocity` (`self.Current Sliding Velocity`) (`self.CharacterMovement`))
      (bind _returnvalue (`KismetSystemLibrary.K2_SetTimer` null "Continue Sliding" 0.01 true))
      (set `self.Continue Sliding Handle` _returnvalue)
      (set `self.Current Angle` (`self.FindCurrentFloorAngleAndDirection`))
      (else
        (goto _label_2)))))

(event `Tracing Floor While Sliding`
  (bind _continue_sliding_handle (`self.Continue Sliding Handle`))
  (`|ExecutionSequence`
    (:`then_0`
      (`self.Check Floor` 4.0)
      (`KismetSystemLibrary.K2_ClearAndInvalidateTimerHandle` (`self.Slide Trace Handle`))
      (if (`KismetSystemLibrary.K2_IsValidTimerHandle` _continue_sliding_handle)
        (`KismetSystemLibrary.K2_ClearAndInvalidateTimerHandle` _continue_sliding_handle))
      (`self.Revert Capsule`)
      (`self.Reset XY Rotation`))
    (:`then_1`
      (`self.Align Player To Floor` 5.0))
    (:`then_2`
      (`self.Check Hit Surface` 0.0 20.0 80.0 "ForOneFrame"
        (:`true`
          (`KismetSystemLibrary.K2_ClearAndInvalidateTimerHandle` (`self.Slide Trace Handle`))
          (`self.Play GetUp Animation`))))))

(event `Revert Capsule`
  (if (not (`NavMovementComponent.IsCrouching` (`self.CharacterMovement`)))
    (bind (_direction _value) (`Timeline|ScaleCapsule` :!via `Reverse` :!label _label_3)
      (:`Update`
        (bind _returnvalue (`KismetMathLibrary.FClamp` _value))
        (`CapsuleComponent.SetCapsuleHalfHeight` (`self.CapsuleComponent`) (`KismetMathLibrary.Lerp` 88.0 34.0 _returnvalue) true)
        (`SceneComponent.K2_SetRelativeLocation` (`self.Mesh`) (`KismetMathLibrary.VLerp` (0.0 0.0 -88.0) (0.0 0.0 -34.0) _returnvalue) false false)))))

(event `Sliding Start`
  (if (> (`KismetMathLibrary.VSize` (`MovementComponent.Velocity` (`self.CharacterMovement`))) 3.0)
    (if (not (and (`AnimInstance.Montage_IsPlaying` (`SkeletalMeshComponent.GetAnimInstance` (`self.Mesh`)) null) (`NavMovementComponent.IsFalling` (`self.CharacterMovement`))))
      (`|ExecutionSequence`
        (:`then_0`
          (set `self.IsSliding` true)
          (`AnimInstance.Montage_Play` (`SkeletalMeshComponent.GetAnimInstance` (`self.Mesh`)) "/Game/MyCharacter/Animation/Montage/Sliding/AM_Sliding.AM_Sliding" 1.0 "MontageLength" 0.0 true))
        (:`then_1`
          (goto _label_3))
        (:`then_2`
          (bind _returnvalue (`KismetSystemLibrary.K2_SetTimerDelegate` (delegate `Tracing Floor While Sliding`) 0.01 true))
          (set `self.Slide Trace Handle` _returnvalue))))))

(event `EnhancedInput|/Game/MyCharacter/Blueprint/Input/InputAction/IA_WeaponChange`
  (params (ActionValue :type Boolean) (ElapsedSeconds :type "Float (double-precision)") (TriggeredSeconds :type "Float (double-precision)") (InputAction :type "InputAction Object Reference" :default "/Game/MyCharacter/Blueprint/Input/InputAction/IA_WeaponChange.IA_WeaponChange"))
  (:`Started`
    (`self.WeaponChangeToNextWeapon`)))

(event `EnhancedInput|/Game/MyCharacter/Blueprint/Input/InputAction/IA_Sliding`
  (params (ActionValue :type Boolean) (ElapsedSeconds :type "Float (double-precision)") (TriggeredSeconds :type "Float (double-precision)") (InputAction :type "InputAction Object Reference" :default "/Game/MyCharacter/Blueprint/Input/InputAction/IA_Sliding.IA_Sliding"))
  (:`Triggered`
    (`self.Sliding Start`)))

(event `EnhancedInput|/Game/MyCharacter/Blueprint/Input/InputAction/IA_Vault`
  (params (ActionValue :type Boolean) (ElapsedSeconds :type "Float (double-precision)") (TriggeredSeconds :type "Float (double-precision)") (InputAction :type "InputAction Object Reference" :default "/Game/MyCharacter/Blueprint/Input/InputAction/IA_Vault.IA_Vault"))
  (:`Triggered`
    (if (and (and (> (`KismetMathLibrary.VSize` (`MovementComponent.Velocity` (`self.CharacterMovement`))) 100.0) (not (`NavMovementComponent.IsFalling` (`self.CharacterMovement`)))) (not (`self.isVaulting`)))
      (bind (_vault_start _vault_middle _vault_land _vault_distance_return) (`self.Vault Trace` 380.0 100.0 45.0 100.0 "ForDuration"))
      (if (`self.Can Vault`)
        (`self.Vault` _vault_start _vault_middle _vault_land _vault_distance_return)))))

(event `ComboEnd`
  ;[1 1 1 1 40] Combo Attack
  (set `self.isAttack` false)
  (set `self.isCombo` false)
  (set `self.ComboCount` 0))

(event `ComboAttack`
  ;[1 1 1 1 40] Combo Attack
  (if (`self.isCombo`)
    (bind _result (`/Engine/EditorBlueprintResources/StandardMacros.IncrementInt` (`self.ComboCount`))
      (:`  `
        (if (not (>= _result 3))
          (switch `int` (`self.ComboCount`)
            (:`1`
              (switch `EWeaponType` (`self.WeaponType`)
                (:`Bared`
                  (`self.PlayAnimMontage` "/Game/MyCharacter/Animation/Montage/Attack/Hands/AM_Punching2_Montage.AM_Punching2_Montage"))
                (:`Sword`
                  (`self.PlayAnimMontage` "/Game/MyCharacter/Animation/Montage/Attack/Sword/AM_Great_Sword_Slash2_Montage.AM_Great_Sword_Slash2_Montage"))))
            (:`2`
              (switch `EWeaponType` (`self.WeaponType`)
                (:`Bared`
                  (`self.PlayAnimMontage` "/Game/MyCharacter/Animation/Montage/Attack/Hands/AM_Punching3_Montage.AM_Punching3_Montage"))
                (:`Sword`
                  (`self.PlayAnimMontage` "/Game/MyCharacter/Animation/Montage/Attack/Sword/AM_Great_Sword_Slash3_Montage.AM_Great_Sword_Slash3_Montage")))))
          (set `self.isCombo` false))))))

(event `EnhancedInput|/Game/MyCharacter/Blueprint/Input/InputAction/IA_Attack`
  (params (ActionValue :type Boolean) (ElapsedSeconds :type "Float (double-precision)") (TriggeredSeconds :type "Float (double-precision)") (InputAction :type "InputAction Object Reference" :default "/Game/MyCharacter/Blueprint/Input/InputAction/IA_Attack.IA_Attack"))
  ;[1 1 1 1 40] Combo Attack
  (:`Started`
    (if (`self.isAttack`)
      (if (not (`self.isCombo`))
        (set `self.isCombo` true))
      (else
        (set `self.isAttack` true)
        (set `self.ComboCount` 0)
        (switch `EWeaponType` (`self.WeaponType`)
          (:`Bared`
            (`self.PlayAnimMontage` "/Game/MyCharacter/Animation/Montage/Attack/Hands/AM_Punching1_Montage.AM_Punching1_Montage"))
          (:`Sword`
            (`self.PlayAnimMontage` "/Game/MyCharacter/Animation/Montage/Attack/Sword/AM_Great_Sword_Slash1_Montage.AM_Great_Sword_Slash1_Montage")))))))

(fn `FindCurrentFloorAngleAndDirection`
  (returns (Angle :type "Float (double-precision)") (`Is Slope Up` :type Boolean))
  (bind (_bblockinghit _binitialoverlap _time _distance _location _impactpoint _normal) (`GameplayStatics.BreakHitResult` (`.HitResult` (break `FindFloorResult` (`CharacterMovementComponent.CurrentFloor` (`self.CharacterMovement`))))))
  (bind (_returnvalue_roll _returnvalue_pitch) (`KismetMathLibrary.BreakRotator` (`KismetMathLibrary.MakeRotFromXY` _normal (`self.GetActorForwardVector`))))
  ;[1 1 1] Find the current floors angle using math and if the current floor is slopping upwards or downwards based on the direction the player is sliding on it.
  (return (`KismetMathLibrary.DegAcos` (`KismetMathLibrary.Dot_VectorVector` _normal (0.0 0.0 1.0))) (> (* _returnvalue_roll _returnvalue_pitch) 0.0)))

(fn `UserConstructionScript`)

(fn `Vault Trace`
  (params (`Initial Trace Length` :type "Float (double-precision)") (`Secondary Trace Z Offset` :type "Float (double-precision)") (`Secondary Trace Gap` :type "Float (double-precision)") (`Landing Position Forward Offset` :type "Float (double-precision)") (DrawDebugType :type "EDrawDebugTrace Enum" :default "None"))
  (returns (`Vault Start` :type "Vector Structure") (`Vault Middle` :type "Vector Structure") (`Vault Land` :type "Vector Structure") (`Vault Distance Return` :type Integer))
  (locals (`Vault Start Location` :type "Vector Structure") (`Vault Middle Location` :type "Vector Structure") (`Vault Land Location` :type "Vector Structure") (`Vault Distance` :type Integer))
  (bind _returnvalue (`self.K2_GetActorLocation`))
  ;[1 1 1] Do a line trace to trace for the object to valut over. if an object is found, te script continues to find the target location. Vault distance is set to 0 so it can be incremented to find the vaulting distance and play different montages based on it.
  (bind (_outhit _returnvalue_2) (`KismetSystemLibrary.LineTraceSingle` :`Start` _returnvalue :`End` (+ _returnvalue (* (`self.GetActorForwardVector`) `Initial Trace Length`)) :`TraceChannel` "TraceTypeQuery1" :`DrawDebugType` DrawDebugType))
  (if _returnvalue_2
    (set `local.Vault Distance` 0)
    ;[1 1 1] Sphere traces used to determine the length of the object and the height.
    (for _index (range 11)
      (`/Engine/EditorBlueprintResources/StandardMacros.IncrementInt` (`local.Vault Distance`)
        (:`  `
          (bind _returnvalue_3 (+ (+ (`.Location` (`GameplayStatics.BreakHitResult` _outhit)) (0.0 0.0 0.0)) (* (`self.GetActorForwardVector`) _index (`local.Secondary Trace Gap`))))
          (bind (_outhit_2 _returnvalue_4) (`KismetSystemLibrary.SphereTraceSingle` :`Start` (+ _returnvalue_3 (`KismetMathLibrary.MakeVector` 0.0 0.0 (`local.Secondary Trace Z Offset`))) :`End` _returnvalue_3 :`Radius` 10.0 :`TraceChannel` "TraceTypeQuery1" :`DrawDebugType` (`local.DrawDebugType`)))
          ;[1 1 1] If it is the first/initial trace then the vault starting location is set and a sphere trace is used to check if there is anything blocking so the vault can be cancelled if there is.
          (if _returnvalue_4
            (if (== _index 0)
              (bind _output_get (set `local.Vault Start Location` (`.ImpactPoint` (`GameplayStatics.BreakHitResult` _outhit_2))))
              (bind _returnvalue_5 (+ _output_get (0.0 0.0 20.0)))
              (bind (_outhit_3 _returnvalue_6) (`KismetSystemLibrary.SphereTraceSingle` :`Start` _returnvalue_5 :`End` _returnvalue_5 :`Radius` 10.0 :`TraceChannel` "TraceTypeQuery1" :`DrawDebugType` (`local.DrawDebugType`)))
              (if _returnvalue_6
                (set `self.Can Vault` false)
                (break))
              (else
                (bind (_bblockinghit _binitialoverlap _time _distance _location _impactpoint _normal _impactnormal _physmat _hitactor _hitcomponent _hitbonename _bonename _hititem _elementindex _faceindex _tracestart _traceend) (`GameplayStatics.BreakHitResult` _outhit_2))
                ;[1 1 1] If the trace is not the initial one then the vault middle/height location is set by setting is every time a trace is done. making the final trace the target middle location.
                (set `local.Vault Middle Location` _impactpoint)
                (bind (_outhit_4 _returnvalue_7) (`KismetSystemLibrary.SphereTraceSingle` :`Start` _tracestart :`End` _tracestart :`Radius` 10.0 :`TraceChannel` "TraceTypeQuery1" :`DrawDebugType` (`local.DrawDebugType`)))
                (if _returnvalue_7
                  (set `self.Can Vault` false))))
            (else
              ;[1 1 1] Find the landing location by doing a line trace downwards from an offset so it is not directly tracing down to the object but to the floor.
              (set `self.Can Vault` true)
              (`|ExecutionSequence`
                (:`then_0`
                  (bind _returnvalue_8 (+ _traceend (* (`self.GetActorForwardVector`) (`local.Landing Position Forward Offset`))))
                  (bind _outhit_5 (`KismetSystemLibrary.LineTraceSingle` :`Start` _returnvalue_8 :`End` (- _returnvalue_8 (0.0 0.0 100.0)) :`TraceChannel` "TraceTypeQuery1" :`DrawDebugType` (`local.DrawDebugType`)))
                  (bind (_outhit_6 _returnvalue_9) (`KismetSystemLibrary.SphereTraceSingle` :`Start` _returnvalue_8 :`End` _returnvalue_8 :`Radius` 20.0 :`TraceChannel` "TraceTypeQuery1" :`DrawDebugType` (`local.DrawDebugType`)))
                  (if _returnvalue_9
                    (set `self.Can Vault` false)
                    (else
                      (set `local.Vault Land Location` (`.Location` (`GameplayStatics.BreakHitResult` _outhit_5))))))
                (:`then_1`
                  (break))))))))
    (return (`local.Vault Start Location`) (`local.Vault Middle Location`) (`local.Vault Land Location`) (`local.Vault Distance`))))

(fn `WeaponChange`
  (params (WeaponType :type "EWeaponType Enum" :default "Bared"))
  (bind _weaponmesh (`self.WeaponMesh`))
  (bind _weaponmesh_2 (`self.WeaponMesh`))
  (bind _output_get (set `self.WeaponType` WeaponType))
  (switch `EWeaponType` _output_get
    (:`Bared`
      (`SkeletalMeshComponent.SetSkeletalMeshAsset` _weaponmesh null)
      (`SceneComponent.SetHiddenInGame` _weaponmesh_2 true false))
    (:`Sword`
      (`SkeletalMeshComponent.SetSkeletalMeshAsset` _weaponmesh "/Game/InfinityBladeWeapons/Weapons/Blade/Swords/Blade_BlackKnight/SK_Blade_BlackKnight.SK_Blade_BlackKnight")
      (`SceneComponent.SetHiddenInGame` _weaponmesh_2 false false)
      (`SceneComponent.K2_AttachToComponent` (`self.WeaponMesh`) (`self.Mesh`) "WeaponSocket" "KeepRelative" "KeepRelative" "KeepRelative" true)
      (`SceneComponent.K2_SetRelativeRotation` (`self.WeaponMesh`) (struct :`Pitch` -80.0 :`Yaw` 137.0 :`Roll` -155.0) false false))))

(fn `WeaponChangeToNextWeapon`
  (bind _returnvalue (+ (`KismetMathLibrary.Conv_ByteToInt` (`self.WeaponType`)) 1))
  (if (>= _returnvalue (`self.WeaponTypeSize`))
    (bind _output_get (set `self.WeaponType` "Bared"))
    (`self.WeaponChange` _output_get)
    (bind _foundwidgets (`WidgetBlueprintLibrary.GetAllWidgetsOfClass` "/Game/MyCharacter/Blueprint/WIdget/WB_UI.WB_UI_C"))
    (`/Game/MyCharacter/Blueprint/WIdget/WB_UI.SetWeaponText` _foundwidgets "주먹")
    (else
      (bind _output_get_2 (set `self.WeaponType` (cast `EWeaponType` (`KismetMathLibrary.Conv_IntToByte` _returnvalue))))
      (`self.WeaponChange` _output_get_2)
      (bind _foundwidgets_2 (`WidgetBlueprintLibrary.GetAllWidgetsOfClass` "/Game/MyCharacter/Blueprint/WIdget/WB_UI.WB_UI_C"))
      (switch `EWeaponType` (`self.WeaponType`)
        (:`Bared`
          (`/Game/MyCharacter/Blueprint/WIdget/WB_UI.SetWeaponText` _foundwidgets_2 "주먹"))
        (:`Sword`
          (`/Game/MyCharacter/Blueprint/WIdget/WB_UI.SetWeaponText` _foundwidgets_2 "대검"))))))